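; Sliding door actor that opens when something overlaps its range or hits it, and closes once nothing overlaps.
; A timeline raises the Door component along Z on opening and reverses to close, with a sound cue for each direction.
; A hit also starts a short timer that attempts the close, which a new overlap cancels.
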(event Custom|CloseDoor
  ;[1 1 1] Si algo entra en el radio de acción de la puerta o es golpeada, se abre... y si deja de haber objetos en el radio de acción (o pasa un tiempo tras haber sido golpeada, y tampoco hay objetos) se cierra.
  (if (== (Utilities|Array|Length (Collision|GetOverlappingActors 0 :!class /Script/Engine.Actor)) 0)
    (Audio|PlaySoundatLocation "/Engine/EditorSounds/GamePreview/EjectFromPlayer_Cue.EjectFromPlayer_Cue" "0, 0, 0" "0, 0, 0" 0.5 1.2 0.0 0 0 0)
    (bind _position (Timeline|DoorOpenTimeline Reverse)
      (:Update
        (Transformation|SetRelativeLocation (Variables|Default|GetDoor) (Math|Vector|MakeVector 0.0 0.0 (Math|Float|Lerp 0.0 5e+02 _position)) false false)))))

(event Collision|EventActorBeginOverlap
  (params (OtherActor :type Actor%20Object%20Reference))
  ;[1 1 1] Si algo entra en el radio de acción de la puerta o es golpeada, se abre... y si deja de haber objetos en el radio de acción (o pasa un tiempo tras haber sido golpeada, y tampoco hay objetos) se cierra.
  (Utilities|Time|ClearandInvalidateTimerbyHandle (stale Collision|EventHit _returnvalue))
  (Audio|PlaySoundatLocation "/Engine/EditorSounds/GamePreview/EjectFromPlayer_Cue.EjectFromPlayer_Cue" (Transformation|GetActorLocation) "0, 0, 0" 1.0 1.0 0.0 0 0 0)
  (bind _position (Timeline|DoorOpenTimeline Play)
    (:Update
      (Transformation|SetRelativeLocation (Variables|Default|GetDoor) (Math|Vector|MakeVector 0.0 0.0 (Math|Float|Lerp 0.0 5e+02 _position)) false false))))

(event Collision|EventActorEndOverlap
  (params (OtherActor :type Actor%20Object%20Reference))
  ;[1 1 1] Si algo entra en el radio de acción de la puerta o es golpeada, se abre... y si deja de haber objetos en el radio de acción (o pasa un tiempo tras haber sido golpeada, y tampoco hay objetos) se cierra.
  (if (== (Utilities|Array|Length (Collision|GetOverlappingActors 0 :!class /Script/Engine.Actor)) 0)
    (Audio|PlaySoundatLocation "/Engine/EditorSounds/GamePreview/EjectFromPlayer_Cue.EjectFromPlayer_Cue" "0, 0, 0" "0, 0, 0" 0.5 1.2 0.0 0 0 0)
    (bind _position (Timeline|DoorOpenTimeline Reverse)
      (:Update
        (Transformation|SetRelativeLocation (Variables|Default|GetDoor) (Math|Vector|MakeVector 0.0 0.0 (Math|Float|Lerp 0.0 5e+02 _position)) false false)))))

(event Collision|EventHit
  (params (MyComp :type Primitive%20Component%20Object%20Reference) (Other :type Actor%20Object%20Reference) (OtherComp :type Primitive%20Component%20Object%20Reference) (bSelfMoved :type Boolean) (HitLocation :type Vector :default "0, 0, 0") (HitNormal :type Vector :default "0, 0, 0") (NormalImpulse :type Vector :default "0, 0, 0") (Hit :type Hit%20Result%20Structure%20%28by%20ref%29))
  ;[1 1 1] Si algo entra en el radio de acción de la puerta o es golpeada, se abre... y si deja de haber objetos en el radio de acción (o pasa un tiempo tras haber sido golpeada, y tampoco hay objetos) se cierra.
  (bind _returnvalue (Utilities|Time|SetTimerbyEvent (delegate Custom|CloseDoor) 2.0))
  (Audio|PlaySoundatLocation "/Engine/EditorSounds/GamePreview/EjectFromPlayer_Cue.EjectFromPlayer_Cue" (Transformation|GetActorLocation) "0, 0, 0" 1.0 1.0 0.0 0 0 0)
  (bind _position (Timeline|DoorOpenTimeline Play)
    (:Update
      (Transformation|SetRelativeLocation (Variables|Default|GetDoor) (Math|Vector|MakeVector 0.0 0.0 (Math|Float|Lerp 0.0 5e+02 _position)) false false))))

(fn ConstructionScript)