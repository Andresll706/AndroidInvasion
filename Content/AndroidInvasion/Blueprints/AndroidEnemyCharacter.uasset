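; Enemy android character that damages the player continuously while overlapping, applying DPS scaled by delta time on Tick between begin and end overlap.
; Impact events decrement Hits; at zero it destroys its capsule, ragdolls the mesh with fire, then explodes and destroys itself after a delay.
; The construction script picks the male or female mannequin mesh and material from IsFemale, and UpdateWalkSpeed sets movement speed.
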(event Collision|EventActorBeginOverlap
  (params (OtherActor :type Actor%20Object%20Reference))
  ;[1 1 1] Mientras esté solapado con el jugador, le hago daño
  (Variables|Default|SetAndroid%20Character (.AsAndroid%20Player%20Character (Utilities|Casting|CastToAndroidPlayerCharacter OtherActor)))
  (Variables|Default|SetDoingDamage true)
  (Audio|PlaySoundatLocation "/Engine/VREditor/Sounds/UI/Laser_Push.Laser_Push" (Transformation|GetActorLocation) "0, 0, 0" 1.0 1.0 0.0 0 0 0))

(event Collision|EventActorEndOverlap
  (params (OtherActor :type Actor%20Object%20Reference))
  ;[1 1 1] Mientras esté solapado con el jugador, le hago daño
  (Variables|Default|SetDoingDamage false)
  (Audio|PlaySoundatLocation "/Engine/VREditor/Sounds/UI/Laser_Pull.Laser_Pull" (Transformation|GetActorLocation) "0, 0, 0" 1.0 1.0 0.0 0 0 0))

(event EventTick
  (params (DeltaSeconds :type Float%20%28single-precision%29))
  ;[1 1 1] Mientras esté solapado con el jugador, le hago daño
  (if (Variables|Default|GetDoingDamage)
    (Game|Damage|ApplyDamage (Variables|Default|GetAndroid%20Character) (* DeltaSeconds (Variables|Default|GetDPS)) 0 0)))

(event EventImpact
  (params (Projectile :type Actor%20Object%20Reference))
  (bind _returnvalue (Transformation|GetActorLocation))
  (bind _mesh (Variables|Character|GetMesh))
  ;[1 1 1] Si me impactan y todavía tengo colisión, pierdo 1 hit...
  ; Cuando no me quedan hits, me destruyo porque me han matado
  ; Si me han matado y tengo malla estática... simulo física en esa malla
  (Utilities|IsValid (Variables|Collision|GetCapsuleComponent)
    (:Is%20Valid
      (bind _result (Math|Integer|DecrementInt (Variables|Default|GetHits))
        (:%20%20
          (if (<= _result 0)
            (Components|DestroyComponent (Variables|Collision|GetCapsuleComponent))
            (Variables|Default|SetDoingDamage false)
            (Audio|PlaySoundatLocation "/Game/StarterContent/Audio/Explosion_Cue.Explosion_Cue" _returnvalue "0, 0, 0" 1.0 1.0 0.0 0 0 0)
            (Utilities|IsValid _mesh
              (:Is%20Valid
                (Physics|SetSimulatePhysics _mesh true)
                (Components|Activation|Activate (Variables|Default|GetFire) false)
                (Audio|PlaySoundatLocation "/Game/StarterContent/Audio/Fire01_Cue.Fire01_Cue" _returnvalue "0, 0, 0" 1.0 1.0 0.0 0 0 0)
                (Utilities|FlowControl|Delay 6.0)
                (Audio|PlaySoundatLocation "/Game/StarterContent/Audio/Explosion_Cue.Explosion_Cue" _returnvalue "0, 0, 0" 0.8 1.0 0.0 0 0 0)
                (Effects|SpawnEmitteratLocation "/Game/StarterContent/Particles/P_Explosion.P_Explosion" _returnvalue "0, 0, 0" "0.800000,0.800000,0.800000")
                (Actor|DestroyActor)))))))))

(fn ConstructionScript
  (bind _mesh (Variables|Character|GetMesh))
  (bind _mesh_2 (Variables|Character|GetMesh))
  (if (Variables|Default|GetIsFemale)
    (Class|SkinnedMeshComponent|SetSkeletalMesh _mesh "/Game/Mannequin/Character/Mesh/SK_Mannequin_Female.SK_Mannequin_Female" true)
    (Rendering|Material|SetMaterial _mesh_2 0 "/Game/AndroidInvasion/Materials/MI_AndroidFemale.MI_AndroidFemale")
    (else
      (Class|SkinnedMeshComponent|SetSkeletalMesh _mesh "/Game/Mannequin/Character/Mesh/SK_Mannequin.SK_Mannequin" true)
      (Rendering|Material|SetMaterial _mesh_2 0 "/Game/AndroidInvasion/Materials/MI_AndroidMale.MI_AndroidMale"))))

(fn UpdateWalkSpeed
  (params (NewWalkSpeed :type Float%20%28single-precision%29))
  (Variables|/Script/Engine.CharacterMovementComponent|SetMaxWalkSpeed (Variables|Character|GetCharacterMovement) NewWalkSpeed))