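; AI controller for the android enemy that runs a behavior tree on possession to drive its response to the player.
; AI perception writes player sightings to the Blackboard as a line-of-sight flag and target actor.
; Other perception updates start a timer that clears both keys, and sensing the player again cancels it.
; A simpler distance-based chase alternative, AICheck, remains in the graph with its looping timer disconnected.
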(event OnTargetPerceptionUpdated(AIPerception)
  (params (Actor :type Actor%20Object%20Reference) (Stimulus :type AI%20Stimulus%20Structure))
  (bind _blackboard (Variables|Default|GetBlackboard))
  ;[1 1 1] Alternativa con IA (BTs y BB), aunque NO LO VAMOS A EXPLICAR TODAVÍA: Ejecuta una serie de tareas, de modo que cuando percibe al jugador, lo persigue... y si no, patrulla en puntos aleatorios
  (if (and (Actor|ActorHasTag Actor "Player") (Utilities|Struct|BreakAIStimulus Stimulus))
    (Utilities|Time|ClearandInvalidateTimerbyHandle (Variables|Default|GetEnemyTimer))
    (AI|Components|Blackboard|SetValueasBool _blackboard (Variables|Default|GetHasLineOfSight) true)
    (AI|Components|Blackboard|SetValueasObject _blackboard (Variables|Default|GetEnemyActor) Actor)
    (else
      (bind _returnvalue (Utilities|Time|SetTimerbyEvent (delegate Custom|StartEnemyTimer) (Variables|Default|GetLineOfSightTimer)))
      (Variables|Default|SetEnemyTimer _returnvalue))))

(event Custom|AICheck
  (bind _returnvalue (Pawn|GetControlledPawn))
  (bind _returnvalue_2 (Game|GetPlayerCharacter 0))
  (bind _returnvalue_3 (Transformation|GetActorLocation _returnvalue_2))
  (bind _returnvalue_4 (Transformation|GetActorLocation _returnvalue))
  ;[1 1 1] Alternativa sin IA: Cada 2 segundos compruebo si estoy a 1 metro del jugador, y si es así, "le ataco" y si no, voy hacia él
  (if (<= (Math|Vector|Distance(Vector) _returnvalue_3 _returnvalue_4) 1e+02)
    ;;[1 1 1] Habría que encontrar la manera de hacer el ataque
    (Transformation|AddActorLocalOffset (Pawn|GetControlledPawn) (- _returnvalue_3 _returnvalue_4) false true)
    (else
      (AI|Navigation|MovetoActor self (Game|GetPlayerCharacter 0) -1.0 true true true 0))))

(event Custom|StartEnemyTimer
  (bind _blackboard (Variables|Default|GetBlackboard))
  ;[1 1 1] Alternativa con IA (BTs y BB), aunque NO LO VAMOS A EXPLICAR TODAVÍA: Ejecuta una serie de tareas, de modo que cuando percibe al jugador, lo persigue... y si no, patrulla en puntos aleatorios
  (AI|Components|Blackboard|SetValueasBool _blackboard (Variables|Default|GetHasLineOfSight) false)
  (AI|Components|Blackboard|SetValueasObject _blackboard (Variables|Default|GetEnemyActor) 0))

(event EventPossess
  (params (PossessedPawn :type Pawn%20Object%20Reference))
  ;[1 1 1] Alternativa con IA (BTs y BB), aunque NO LO VAMOS A EXPLICAR TODAVÍA: Ejecuta una serie de tareas, de modo que cuando percibe al jugador, lo persigue... y si no, patrulla en puntos aleatorios
  (AI|RunBehaviorTree "/Game/AndroidInvasion/AI/AndroidEnemyBT.AndroidEnemyBT"))

(event EventBeginPlay
  ;[1 1 1] Alternativa sin IA: Cada 2 segundos compruebo si estoy a 1 metro del jugador, y si es así, "le ataco" y si no, voy hacia él
)

(fn ConstructionScript)