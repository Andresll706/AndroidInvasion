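; Player controller for Android Invasion that drives the possessed AndroidPlayerCharacter and relays game results to the HUD.
; It caches the pawn on possess, then forwards look, movement, jump and run input to it.
; Number keys select the weapon that Fire uses, normal shots or grenades, and Dash spends stamina to launch the character forward.
; Win and GameOver events open AndroidHUD menus, though only GameOver shows the mouse cursor.
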(event Custom|GameOver
  ;[1 1 1] Cuando me avisen de que he muerto, muestro el ratón (me faltaría hacer foco en los botones) y saco el menú de partida perdida
  (Variables|Default|SetbShowMouseCursor true)
  (Default|ShowGameOver (CallFunction|GetAndroidHUD)))

(event Custom|Win
  ;[1 1 1] Cuando me avisen de que he ganado, muestro el ratón (me faltaría hacer foco en los botones) y saco el menú de victoria
  (Default|ShowWinMenu (CallFunction|GetAndroidHUD)))

(event EventPossess
  (params (PossessedPawn :type Pawn%20Object%20Reference))
  ;[1 1 1] Android Player Controller - Cuando posea algo, asumo que es el AndroidCharacter y me lo guardo (en realidad esto lo podría obviar)
  (Variables|Default|SetAndroidCharacter (.AsAndroid%20Player%20Character (Utilities|Casting|CastToAndroidPlayerCharacter PossessedPawn))))

(event Input|ActionEvents|InputActionRun
  (params (Key :type Key%20Structure :default "None"))
  (bind _androidcharacter (Variables|Default|GetAndroidCharacter))
  ;[1 1 1] Añadir la posibilidad de correr y gastar energia (recuperarla por no correr)
  (:Pressed
    (Variables|/Game/AndroidInvasion/Blueprints/AndroidPlayerCharacter.AndroidPlayerCharacter_C|SetIsRunning _androidcharacter true))
  (:Released
    (Variables|/Game/AndroidInvasion/Blueprints/AndroidPlayerCharacter.AndroidPlayerCharacter_C|SetIsRunning _androidcharacter false)))

(event Input|ActionEvents|InputActionDash
  (params (Key :type Key%20Structure :default "None"))
  (bind _androidcharacter (Variables|Default|GetAndroidCharacter))
  (bind _returnvalue (Transformation|GetActorForwardVector _androidcharacter))
  (bind (_x _y _z) (Math|Vector|BreakVector _returnvalue))
  ;[1 1 1] Dash
  (:Pressed
    (if (> (- (Variables|/Game/AndroidInvasion/Blueprints/AndroidPlayerCharacter.AndroidPlayerCharacter_C|GetStamina (Variables|Default|GetAndroidCharacter)) 2e+01) 0.0)
      (Variables|/Game/AndroidInvasion/Blueprints/AndroidPlayerCharacter.AndroidPlayerCharacter_C|SetStamina (Variables|Default|GetAndroidCharacter) (- (Variables|/Game/AndroidInvasion/Blueprints/AndroidPlayerCharacter.AndroidPlayerCharacter_C|GetStamina (Variables|Default|GetAndroidCharacter)) 2e+01))
      (Character|LaunchCharacter (Variables|Default|GetAndroidCharacter) (Math|Vector|MakeVector (* _x 5e+03) (* _y 5e+03) _z) false false))))

(event Input|ActionEvents|InputActionJump
  (params (Key :type Key%20Structure :default "None"))
  (bind _androidcharacter (Variables|Default|GetAndroidCharacter))
  ;[1 1 1] Salto
  (:Pressed
    (Character|Jump _androidcharacter))
  (:Released
    (Character|StopJumping _androidcharacter)))

(event Input|ActionEvents|InputActionFire
  (params (Key :type Key%20Structure :default "None"))
  (bind _androidcharacter (Variables|Default|GetAndroidCharacter))
  ;[1 1 1] Si pulsan disparar, le digo al cuerpo que dispare
  (:Pressed
    (if (== (Variables|/Game/AndroidInvasion/Blueprints/AndroidPlayerCharacter.AndroidPlayerCharacter_C|GetWeapon (Variables|Default|GetAndroidCharacter)) 1)
      (Default|Fire _androidcharacter)
      (else
        (Default|FireGranades _androidcharacter)))))

(event Input|AxisEvents|InputAxisTurn
  (params (AxisValue :type Float%20%28single-precision%29))
  ;[1 1 1] Rotaciones con el ratón
  (Pawn|Input|AddControllerYawInput (Variables|Default|GetAndroidCharacter) AxisValue))

(event Input|AxisEvents|InputAxisLookUp
  (params (AxisValue :type Float%20%28single-precision%29))
  ;[1 1 1] Rotaciones con el ratón
  (Pawn|Input|AddControllerPitchInput (Variables|Default|GetAndroidCharacter) AxisValue))

(event Input|AxisEvents|InputAxisMoveForward
  (params (AxisValue :type Float%20%28single-precision%29))
  (bind _androidcharacter (Variables|Default|GetAndroidCharacter))
  ;[1 1 1] Movimiento con el stick (o teclado)
  (Pawn|Input|AddMovementInput _androidcharacter (Transformation|GetActorForwardVector _androidcharacter) AxisValue false))

(event Input|AxisEvents|InputAxisMoveRight
  (params (AxisValue :type Float%20%28single-precision%29))
  (bind _androidcharacter (Variables|Default|GetAndroidCharacter))
  ;[1 1 1] Movimiento con el stick (o teclado)
  (Pawn|Input|AddMovementInput _androidcharacter (Transformation|GetActorRightVector _androidcharacter) AxisValue false))

(event Input|AxisEvents|InputAxisTurnRate
  (params (AxisValue :type Float%20%28single-precision%29))
  (bind _androidcharacter (Variables|Default|GetAndroidCharacter))
  ;[1 1 1] Rotaciones con el stick (o teclado)
  (Pawn|Input|AddControllerYawInput _androidcharacter (* AxisValue (Variables|/Game/AndroidInvasion/Blueprints/AndroidPlayerCharacter.AndroidPlayerCharacter_C|GetBaseTurnRate _androidcharacter) (Utilities|Time|GetWorldDeltaSeconds))))

(event Input|AxisEvents|InputAxisLookUpRate
  (params (AxisValue :type Float%20%28single-precision%29))
  (bind _androidcharacter (Variables|Default|GetAndroidCharacter))
  ;[1 1 1] Rotaciones con el stick (o teclado)
  (Pawn|Input|AddControllerPitchInput _androidcharacter (* AxisValue (Variables|/Game/AndroidInvasion/Blueprints/AndroidPlayerCharacter.AndroidPlayerCharacter_C|GetBaseLookUpRate _androidcharacter) (Utilities|Time|GetWorldDeltaSeconds))))

(event Input|KeyboardEvents|1
  (params (Key :type Key%20Structure :default "None"))
  ;[1 1 1] Cambiar de proyectiles entre granadas y munición normal (llevar la cuenta aparte
  (:Pressed
    (Variables|/Game/AndroidInvasion/Blueprints/AndroidPlayerCharacter.AndroidPlayerCharacter_C|SetWeapon (Variables|Default|GetAndroidCharacter) 1)))

(event Input|KeyboardEvents|2
  (params (Key :type Key%20Structure :default "None"))
  ;[1 1 1] Cambiar de proyectiles entre granadas y munición normal (llevar la cuenta aparte
  (:Pressed
    (Variables|/Game/AndroidInvasion/Blueprints/AndroidPlayerCharacter.AndroidPlayerCharacter_C|SetWeapon (Variables|Default|GetAndroidCharacter) 2)))

(fn ConstructionScript)

(fn GetAndroidHUD
  ;[1 1 1] Devuelve el HUD, asumiendo que siempre es un Android HUD
  (return (.AsAndroid%20HUD (Utilities|Casting|CastToAndroidHUD (HUD|GetHUD)))))