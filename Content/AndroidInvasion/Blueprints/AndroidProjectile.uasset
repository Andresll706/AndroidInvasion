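; AndroidProjectile is a projectile actor that resolves its own collisions in the Hit event.
; It calls Impact on any Android it strikes, passing itself as the argument.
; A physics-simulating hit component receives an impulse equal to the projectile's velocity, applied at the projectile's location.
; Any valid hit component also triggers a quiet, high-pitched explosion sound and destroys the projectile.
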(event Collision|EventHit
  (params (MyComp :type Primitive%20Component%20Object%20Reference) (Other :type Actor%20Object%20Reference) (OtherComp :type Primitive%20Component%20Object%20Reference) (bSelfMoved :type Boolean) (HitLocation :type Vector :default "0, 0, 0") (HitNormal :type Vector :default "0, 0, 0") (NormalImpulse :type Vector :default "0, 0, 0") (Hit :type Hit%20Result%20Structure%20%28by%20ref%29))
  ;[1 1 1] Cuando choco contra algo, si es un Prototipo, IMPACTARLO... si no, si es un cuerpo físico, empujarlo... y si no, pues nada
  (bind _asandroid (Utilities|Casting|CastToAndroid Other)
    (:then
      (Default|Impact _asandroid self))
    (:CastFailed
      _))
  (Utilities|IsValid OtherComp
    (:Is%20Valid
      (if (Physics|IsSimulatingPhysics OtherComp "None")
        (Physics|AddImpulseatLocation OtherComp (Transformation|GetVelocity) (Transformation|GetActorLocation) "None"))
      (Audio|PlaySoundatLocation "/Game/StarterContent/Audio/Explosion_Cue.Explosion_Cue" (Transformation|GetActorLocation) "0, 0, 0" 0.3 2.0 0.0 0 0 0)
      (Actor|DestroyActor))))

(fn ConstructionScript)