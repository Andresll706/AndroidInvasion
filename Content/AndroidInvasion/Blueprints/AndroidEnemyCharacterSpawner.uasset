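; Destructible spawner actor that periodically produces enemy androids in the AndroidInvasion game.
; After a short delay at BeginPlay, a looping timer spawns an AndroidEnemyCharacter of random gender at the child actor's transform and plays an eject sound.
; Each Impact event decrements Hits, and at zero the spawner plays explosion effects and destroys itself.
; Spawning has no population cap, which the author's note flags as still to add.
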(event Custom|SpawnAndroidEnemy
  ;[1 1 1] Al comienzo del juego, establece una alarma cada SpawnTime segundos. Cuando toca, elige un sexo al azar y crear un androide enemigo de ese tipo
  ; Hay que añadir un control para no generar infinitos robots, cada generador puede controlar lo que ha generado él, o haber un control general...
  (Game|SpawnActorfromClass "/Game/AndroidInvasion/Blueprints/AndroidEnemyCharacter.AndroidEnemyCharacter_C" (Transformation|GetWorldTransform (Variables|Default|GetChildActor)) "Undefined" 0 (Math|Random|RandomBool) 0)
  (Audio|PlaySoundatLocation "/Engine/EditorSounds/GamePreview/EjectFromPlayer_Cue.EjectFromPlayer_Cue" (Transformation|GetActorLocation) "0, 0, 0" 2.0 3.0 0.0 0 0 0))

(event EventBeginPlay
  ;[1 1 1] Al comienzo del juego, establece una alarma cada SpawnTime segundos. Cuando toca, elige un sexo al azar y crear un androide enemigo de ese tipo
  ; Hay que añadir un control para no generar infinitos robots, cada generador puede controlar lo que ha generado él, o haber un control general...
  (Utilities|FlowControl|Delay 1.0)
  (Utilities|Time|SetTimerbyEvent (delegate Custom|SpawnAndroidEnemy) (Variables|Default|GetSpawnTime) true))

(event EventImpact
  (params (Projectile :type Actor%20Object%20Reference))
  (bind _returnvalue (Transformation|GetActorLocation))
  ;[1 1 1] Si me disparan lo suficiente, exploto
  (Utilities|IsValid self
    (:Is%20Valid
      (bind _result (Math|Integer|DecrementInt (Variables|Default|GetHits))
        (:%20%20
          (if (<= _result 0)
            (Audio|PlaySoundatLocation "/Game/StarterContent/Audio/Explosion_Cue.Explosion_Cue" _returnvalue "0, 0, 0" 1.0 1.0 0.0 0 0 0)
            (Effects|SpawnEmitteratLocation "/Game/StarterContent/Particles/P_Explosion.P_Explosion" _returnvalue)
            (Actor|DestroyActor)))))))

(fn ConstructionScript)