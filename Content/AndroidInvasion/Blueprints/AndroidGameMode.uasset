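; Game mode for Android Invasion that runs each level's win, loss and difficulty rules.
; On BeginPlay it counts AndroidPrototype actors and divides enemy spawner SpawnTime by the game instance's level, with a one-second floor.
; PrototypeDestroyed increments TargetsLeft until it matches the total, then calls the controller's Win and destroys the "ExitFloor"-tagged mesh to open the exit.
; PlayerDead pauses, resets the game instance for permadeath, and triggers GameOver.
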(event Custom|PrototypeDestroyed
  (bind _targetsleft (Variables|Default|GetTargetsLeft))
  ;[1 1 1] Cuando se destruye un prototipo, se reduce 1 de la cantidad de los que quedan... y si llega a 0, le digo al controlador que ha ganado, y además también hago un cambio en el mapa: busco el primer actor etiquetado como "ExitFloor" y lo elimino, para dejar acceso libre a la salida
  (Math|Integer|IncrementInt _targetsleft
    (:%20%20
      (if (== _targetsleft (Variables|Default|GetTotalTargets))
        (Audio|PlaySound2D "/Game/StarterContent/Audio/Starter_Music_Cue.Starter_Music_Cue" 1.0 1.0 0.0 0 0)
        (Default|Win (CallFunction|GetAndroidPlayerController))
        (bind _outactors (Actor|GetAllActorsOfClasswithTag "/Script/Engine.StaticMeshActor" "ExitFloor"))
        (Audio|PlaySoundatLocation "/Game/StarterContent/Audio/Collapse_Cue.Collapse_Cue" (Transformation|GetActorLocation (Utilities|Array|Get(acopy) _outactors)) "0, 0, 0" 0.5 1.0 0.0 0 0 0)
        (Actor|DestroyActor (Utilities|Array|Get(acopy) _outactors))))))

(event Custom|PlayerDead
  ;[1 1 1] Cuando matan al jugador, pauso, reinicio el nivel por el que vamos (¡permadeth, otra vez al nivel inicial!) y le digo al controlador que ha perdido.
  (Audio|PlaySound2D "/Game/StarterContent/Audio/Explosion_Cue.Explosion_Cue" 4.0 0.5 0.0 0 0)
  (Game|SetGamePaused true)
  (Default|Reset (CallFunction|GetAndroidGameInstance))
  (Default|GameOver (CallFunction|GetAndroidPlayerController)))

(event EventBeginPlay
  ;[1 1 1] Android Game Mode - Nada más empezar un nivel, contabilizo todos los prototipos androides que hay, y guardo el valor total.
  ; Además se ajusta la dificultad según el número de nivel (por ahora únicamente se divide el tiempo de los generadores entre el número del nivel (manteniendo un lapso mínimo de 1 segundo entre generación y generación)
  (bind _outactors (Actor|GetAllActorsOfClass "/Game/AndroidInvasion/Blueprints/AndroidPrototype.AndroidPrototype_C"))
  (Variables|Default|SetTotalTargets (Utilities|Array|Length _outactors))
  (bind _outactors_2 (Actor|GetAllActorsOfClass "/Game/AndroidInvasion/Blueprints/AndroidEnemyCharacterSpawner.AndroidEnemyCharacterSpawner_C"))
  (for _array_element _outactors_2
    (Variables|/Game/AndroidInvasion/Blueprints/AndroidEnemyCharacterSpawner.AndroidEnemyCharacterSpawner_C|SetSpawnTime _array_element (Math|Float|Max(Float) (/ (Variables|/Game/AndroidInvasion/Blueprints/AndroidEnemyCharacterSpawner.AndroidEnemyCharacterSpawner_C|GetSpawnTime _array_element) (Math|Conversions|ToFloat(Integer) (Math|Integer|Max(Integer) (Variables|/Game/AndroidInvasion/Blueprints/AndroidGameInstance.AndroidGameInstance_C|GetLevel (CallFunction|GetAndroidGameInstance)) 1))) 1.0))))

(fn ConstructionScript)