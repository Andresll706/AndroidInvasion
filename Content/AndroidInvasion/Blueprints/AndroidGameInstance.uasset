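; AndroidGameInstance is the game instance for Android Invasion, holding the current level and persisting it across sessions.
; Load reads the AndroidSaveGame from the save slot and copies its level, leaving the current one untouched if none exists.
; Save writes the level into a new save object in that slot.
; Reset zeroes the level and saves immediately, overwriting prior progress.
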(event Custom|Save
  ;[1 1 1] Guardar partida es crear el objeto "partida guardada" y meter lo que quiera guardar del game instance allí (en este caso es trivial: únicamente la variable nivel)
  (bind _returnvalue (SaveGame|CreateSaveGameObject "/Game/AndroidInvasion/Blueprints/AndroidSaveGame.AndroidSaveGame_C"))
  (Variables|/Game/AndroidInvasion/Blueprints/AndroidSaveGame.AndroidSaveGame_C|SetSaveLevel _returnvalue (Variables|Default|GetLevel))
  (SaveGame|SaveGametoSlot _returnvalue (Variables|Default|GetSave%20Game%20Slot)))

(event Custom|Load
  ;[1 1 1] Cargar partida es simplemente ver si hay una partida guardada en el slot (no es NULA y el casting a AndroidSaveGame funciona), actualiza game instance con la información que haya dentro. Si no, no se hace nada (el nivel se queda como está)
  (bind _returnvalue (SaveGame|LoadGamefromSlot (Variables|Default|GetSave%20Game%20Slot)))
  (bind _asandroid_save_game (Utilities|Casting|CastToAndroidSaveGame _returnvalue))
  (Variables|Default|SetLevel (Variables|/Game/AndroidInvasion/Blueprints/AndroidSaveGame.AndroidSaveGame_C|GetSaveLevel _asandroid_save_game)))

(event Custom|Reset
  ;[1 1 1] Reestablecer el juego es poner el nivel a 0 y guardar partida además, machacando lo que hubiésemos avanzado
  (Variables|Default|SetLevel 0)
  (CallFunction|Save))