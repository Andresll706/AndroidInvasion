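; AndroidPrototype is a destructible android in the Android Invasion game that reacts to being hit.
; Its Impact event runs only while the skeletal mesh is not yet simulating physics, so the destruction is not repeated.
; It plays explosion and fire sounds, turns the skeleton into a physics ragdoll and swaps two spark effects for fire.
; It then notifies AndroidGameMode that a prototype has been destroyed.
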(event EventImpact
  (params (Projectile :type Actor%20Object%20Reference))
  (bind _returnvalue (Transformation|GetActorLocation))
  ;[1 1 1] Si recibo un impacto (y aún no estoy simulando física), empiezo a simular físicas en mi esqueleto, activo el fuego y aviso al Game Mode
  (if (not (Physics|IsSimulatingPhysics (Variables|Default|GetSkeletalMeshComponent) "None"))
    (Audio|PlaySoundatLocation "/Game/StarterContent/Audio/Explosion_Cue.Explosion_Cue" _returnvalue "0, 0, 0" 3.0 1.0 0.0 0 0 0)
    (Audio|PlaySoundatLocation "/Game/StarterContent/Audio/Fire01_Cue.Fire01_Cue" _returnvalue "0, 0, 0" 2.0 1.0 0.0 0 0 0)
    (Physics|SetSimulatePhysics (Variables|Default|GetSkeletalMeshComponent) true)
    (Components|Activation|Deactivate (Variables|Default|GetSparks1))
    (Components|Activation|Deactivate (Variables|Default|GetSparks2))
    (Components|Activation|Activate (Variables|Default|GetFire) false)
    (Default|PrototypeDestroyed (.AsAndroid%20Game%20Mode (Utilities|Casting|CastToAndroidGameMode (Game|GetGameMode))))))

(fn ConstructionScript)