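; BP_AmunitionBullets is an ammunition pickup that reloads the bullets of the player character.
; On actor overlap it casts the other actor to AndroidPlayerCharacter and ignores anything else.
; It adds ReloadBullets to the character's Bullets, capped at MaxBullets, then destroys itself, even if the player is already full.
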(event EventBeginPlay)

(event Collision|EventActorBeginOverlap
  (params (OtherActor :type Actor%20Object%20Reference))
  ;[1 1 1] Reload Bullets
  (bind _asandroid_player_character (Utilities|Casting|CastToAndroidPlayerCharacter OtherActor))
  (if (> (+ (Variables|/Game/AndroidInvasion/Blueprints/AndroidPlayerCharacter.AndroidPlayerCharacter_C|GetBullets _asandroid_player_character) (Variables|Default|GetReloadBullets)) (Variables|/Game/AndroidInvasion/Blueprints/AndroidPlayerCharacter.AndroidPlayerCharacter_C|GetMax%20Bullets _asandroid_player_character))
    (Variables|/Game/AndroidInvasion/Blueprints/AndroidPlayerCharacter.AndroidPlayerCharacter_C|SetBullets _asandroid_player_character (Variables|/Game/AndroidInvasion/Blueprints/AndroidPlayerCharacter.AndroidPlayerCharacter_C|GetMax%20Bullets _asandroid_player_character))
    (Actor|DestroyActor)
    (else
      (Variables|/Game/AndroidInvasion/Blueprints/AndroidPlayerCharacter.AndroidPlayerCharacter_C|SetBullets _asandroid_player_character (+ (Variables|/Game/AndroidInvasion/Blueprints/AndroidPlayerCharacter.AndroidPlayerCharacter_C|GetBullets _asandroid_player_character) (Variables|Default|GetReloadBullets)))
      (Actor|DestroyActor))))

(event EventTick
  (params (DeltaSeconds :type Float%20%28single-precision%29)))

(fn ConstructionScript)