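; AndroidHUD is the Android Invasion HUD, handling the intro cinematic, crosshair, header, level notice and end-of-game menus.
; On BeginPlay below level 2, it plays the IntroMaster sequence with game input disabled and zero player gravity, restoring both after a delay.
; It then adds the UMG header and briefly shows level info, while DrawHUD draws a centered crosshair outside cinematics.
; Callable events show a persistent win menu or game-over menu, which replaces it.
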(event Custom|ShowGameOver
  ;[1 1 1] Cuando me lo pidan, muestro el menú de partida perdida (intento quitar el de victoria si está puesto, para que no estén ambos)
  (CallFunction|RemoveWinMenu)
  (bind _returnvalue (UserInterface|CreateWidget "/Game/AndroidInvasion/UI/GameOverMenu.GameOverMenu_C"))
  (UserInterface|Viewport|AddtoViewport _returnvalue 0))

(event Custom|Show%20Win%20Menu
  ;[1 1 1] Cuando me lo pidan, muestro el menú de victoria (no impide el juego y se queda ahí, persistente)
  (bind _returnvalue (UserInterface|CreateWidget "/Game/AndroidInvasion/UI/WinMenu.WinMenu_C"))
  (UserInterface|Viewport|AddtoViewport _returnvalue 0)
  (Variables|Default|SetWinMenu true))

(event Custom|Remove%20Win%20Menu
  ;[1 1 1] Intentar quitar el menú de victoria si está puesto
  (if (Variables|Default|GetWinMenu)
    (Widget|RemovefromParent (stale Custom|Show%20Win%20Menu _returnvalue))))

(event EventBeginPlay
  ;[1 1 1] Al comenzar el jueg, si el nivel es inferior al 2, toca cinemática: se inhabilita la entrada, se pone gravedad a cero (para dejar al personaje en el aire) y se hace la cinemática.
  ; Luego, ya se pone el HUD normal, la parte hecha con UMG... y al ratito un mensaje informando del nivel en el que estás (debería transicionar poco a poco, pero bueno)
  (if (< (Variables|/Game/AndroidInvasion/Blueprints/AndroidGameInstance.AndroidGameInstance_C|GetLevel (CallFunction|GetAndroidGameInstance)) 2)
    (Variables|Default|SetCinematics true)
    (Input|SetInputModeUIOnly (CallFunction|GetAndroidPlayerController) 0 "DoNotLock")
    (Variables|/Script/Engine.CharacterMovementComponent|SetGravityScale (Variables|/Script/Engine.Character|GetCharacterMovement (CallFunction|GetAndroidPlayerCharacter)) 0.0)
    (Audio|PlaySound2D "/Game/StarterContent/Audio/Collapse01.Collapse01" 1.0 0.1 0.0 0 0)
    (bind _returnvalue (Sequencer|Player|CreateLevelSequencePlayer "/Game/Cinematics/Sequences/Intro/IntroMaster.IntroMaster"))
    (Sequencer|Player|Play _returnvalue :!class /Script/MovieScene.MovieSceneSequencePlayer)
    (Utilities|FlowControl|Delay 6.0)
    (Variables|/Script/Engine.CharacterMovementComponent|SetGravityScale (Variables|/Script/Engine.Character|GetCharacterMovement (CallFunction|GetAndroidPlayerCharacter)) 1.0)
    (Input|SetInputModeGameOnly (CallFunction|GetAndroidPlayerController))
    (Variables|Default|SetCinematics false))
  (bind _returnvalue_2 (UserInterface|CreateWidget "/Game/AndroidInvasion/UI/HUDHeader.HUDHeader_C"))
  (UserInterface|Viewport|AddtoViewport _returnvalue_2 0)
  (Utilities|FlowControl|Delay 2.0)
  (bind _returnvalue_3 (UserInterface|CreateWidget "/Game/AndroidInvasion/UI/LevelInfo.LevelInfo_C"))
  (UserInterface|Viewport|AddtoViewport _returnvalue_3 0)
  (Utilities|FlowControl|Delay 2.0)
  (Widget|RemovefromParent _returnvalue_3))

(event EventDrawHUD
  (params (SizeX :type Integer) (SizeY :type Integer))
  ;[1 1 1] Dibujo mediante Slate una mirilla en el centro de la escena (siempre que no esté mostrando cinemáticas)
  (if (not (Variables|Default|GetCinematics))
    (Canvas|DrawTexture "/Game/AndroidInvasion/Textures/AndroidCrosshair.AndroidCrosshair" (Math|Conversions|ToFloat(Integer) (/ SizeX 2)) (Math|Conversions|ToFloat(Integer) (/ SizeY 2)) 32.0 32.0 0.0 0.0 1.0 1.0 (Utilities|Struct|MakeLinearColor 1.0 1.0 1.0 1.0) "BLEND_Translucent" 1.0 true)))

(fn ConstructionScript)