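; First-person player character for AndroidInvasion, handling health, shooting, grenades and stamina-based sprinting.
; Fire and FireGranades spend their ammo, play the fire montage and spawn an AndroidProjectile or AndroidGrenade ahead along the camera rotation, with sound.
; Tick switches walk speed by IsRunning, draining or regenerating stamina per frame without delta-time scaling.
; Damage reduces health and notifies AndroidGameMode at zero; construction snaps the gun to the GripPoint socket.
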(event Custom|Fire
  (bind _firstpersoncamera (Variables|MyCharacter|GetFirstPersonCamera))
  (bind _returnvalue (Transformation|GetWorldRotation _firstpersoncamera))
  ;[1 1 1] Disparar proyectil (de munición normal, podría hacerse lo mismo sean granadas o proyectiles... o bien usar raycast para munición
  (if (> (Variables|Default|GetBullets) 0)
    (bind _result (Math|Integer|DecrementInt (Variables|Default|GetBullets))
      (:%20%20
        (Variables|Default|SetBullets _result)
        (Animation|Montage|MontagePlay (Components|SkeletalMesh|GetAnimInstance (Variables|MyCharacter|GetMesh2P)) "/Game/FirstPerson/Animations/FirstPersonFire_Montage.FirstPersonFire_Montage" 1.0 "MontageLength" 0.0 true)
        (bind _returnvalue_2 (Game|SpawnActorfromClass "/Game/AndroidInvasion/Blueprints/AndroidProjectile.AndroidProjectile_C" (Math|Transform|MakeTransform (+ (Transformation|GetWorldLocation (Variables|Default|GetSphere)) (Math|Vector|RotateVector (Variables|Default|GetGunOffset) _returnvalue)) _returnvalue) "AlwaysSpawn" 0 0)) ; Spawn projectile
        (Utilities|IsValid _returnvalue_2
          (:Is%20Valid
            (Audio|PlaySoundatLocation "/Engine/VREditor/Sounds/UI/Laser_Push.Laser_Push" (Transformation|GetActorLocation) "0, 0, 0" 2.0 1.0 0.0 0 0 0) ; Play firing sound
          ))))))

(event Custom|FireGranades
  (bind _firstpersoncamera (Variables|MyCharacter|GetFirstPersonCamera))
  (bind _returnvalue (Transformation|GetWorldRotation _firstpersoncamera))
  ;[1 1 1] Fire granades
  (if (> (Variables|Default|GetGrenades) 0)
    (bind _result (Math|Integer|DecrementInt (Variables|Default|GetGrenades))
      (:%20%20
        (Variables|Default|SetGrenades _result)
        (Animation|Montage|MontagePlay (Components|SkeletalMesh|GetAnimInstance (Variables|MyCharacter|GetMesh2P)) "/Game/FirstPerson/Animations/FirstPersonFire_Montage.FirstPersonFire_Montage" 1.0 "MontageLength" 0.0 true)
        (bind _returnvalue_2 (Game|SpawnActorfromClass "/Game/AndroidInvasion/Blueprints/AndroidGrenade.AndroidGrenade_C" (Math|Transform|MakeTransform (+ (Transformation|GetWorldLocation (Variables|Default|GetSphere)) (Math|Vector|RotateVector (Variables|Default|GetGunOffset) _returnvalue)) _returnvalue) "AlwaysSpawn" 0 0)) ; Spawn projectile
        (Utilities|IsValid _returnvalue_2
          (:Is%20Valid
            (Audio|PlaySoundatLocation "/Game/StarterContent/Audio/Explosion01.Explosion01" (Transformation|GetActorLocation) "0, 0, 0" 2.0 1.0 0.0 0 0 0) ; Play firing sound
          ))))))

(event Game|Damage|EventAnyDamage
  (params (Damage :type Float%20%28single-precision%29) (DamageType :type Damage%20Type%20Object%20Reference) (InstigatedBy :type Controller%20Object%20Reference) (DamageCauser :type Actor%20Object%20Reference))
  ;[1 1 1] Si recibo daño, lo descuento de mi salud... y si llega a ser cero o menos, aviso al GM que me muero
  (bind _output_get (Variables|Default|SetHealth (- (Variables|Default|GetHealth) Damage)))
  (if (<= _output_get 0.0)
    (Default|PlayerDead (.AsAndroid%20Game%20Mode (Utilities|Casting|CastToAndroidGameMode (Game|GetGameMode))))))

(event EventTick
  (params (DeltaSeconds :type Float%20%28single-precision%29))
  (bind _charactermovement (Variables|Character|GetCharacterMovement))
  (if (Variables|Default|GetIsRunning)
    ;[1 1 1] Running
    (if (>= (- (Variables|Default|GetStamina) 0.5) 0.0)
      (bind _output_get (Variables|Default|SetStamina (- (Variables|Default|GetStamina) 0.5)))
      (Variables|/Script/Engine.CharacterMovementComponent|SetMaxWalkSpeed _charactermovement 1e+03)
      (else
        (Variables|/Script/Engine.CharacterMovementComponent|SetMaxWalkSpeed _charactermovement 6e+02)))
    (else
      ;[1 1 1] Walk and recover stamina
      (Variables|/Script/Engine.CharacterMovementComponent|SetMaxWalkSpeed (Variables|Character|GetCharacterMovement) 6e+02)
      (bind _output_get_2 (Variables|Default|SetStamina (+ (Variables|Default|GetStamina) 0.1)))
      (if (> _output_get_2 1e+02)
        (Variables|Default|SetStamina 1e+02)))))

(fn ConstructionScript
  (Transformation|AttachComponentToComponent (Variables|Default|GetFP_Gun) (Variables|MyCharacter|GetMesh2P) "GripPoint" "SnapToTarget" "SnapToTarget" "SnapToTarget" true))