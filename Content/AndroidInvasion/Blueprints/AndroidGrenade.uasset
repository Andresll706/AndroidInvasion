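; AndroidGrenade is a timed grenade actor that damps nothing on contact but pushes physics bodies it hits with an impulse from its velocity.
; After a Duration delay from BeginPlay it plays explosion particles and sound, then checks overlapping actors.
; Overlapping Androids receive Impact, while other physics-simulating actors get a radial impulse.
; The grenade destroys itself only in the Android branch, so it persists when none overlap.
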(event EventBeginPlay
  (bind _returnvalue (Transformation|GetActorLocation))
  ;[1 1 1] REVISAR: Nada más empezar a existir, cuento Duration segundos y exploto, con partículas, sonido e impactando a todos los androides con los que esté solapado
  (Utilities|FlowControl|Delay (Variables|Default|GetDuration))
  (Components|Activation|Activate (Variables|Default|GetExplosionPS) false)
  (Audio|PlaySoundatLocation "/Game/StarterContent/Audio/Explosion01.Explosion01" _returnvalue "0, 0, 0" 1.0 1.0 0.0 0 0 0)
  (for _array_element (Collision|GetOverlappingActors 0 :!class /Script/Engine.Actor)
    (bind _asandroid (Utilities|Casting|CastToAndroid _array_element)
      (:then
        (Default|Impact _asandroid self)
        (Actor|DestroyActor))
      (:CastFailed
        (if (Physics|IsSimulatingPhysics (Variables|/Script/Engine.Actor|GetRootComponent _array_element) "None")
          (Physics|AddRadialImpulse (.AsPrimitive%20Component (Utilities|Casting|CastToPrimitiveComponent (Variables|/Script/Engine.Actor|GetRootComponent _array_element))) _returnvalue 5e+02 3e+02 "RIF_Constant" false))))))

(event Collision|EventHit
  (params (MyComp :type Primitive%20Component%20Object%20Reference) (Other :type Actor%20Object%20Reference) (OtherComp :type Primitive%20Component%20Object%20Reference) (bSelfMoved :type Boolean) (HitLocation :type Vector :default "0, 0, 0") (HitNormal :type Vector :default "0, 0, 0") (NormalImpulse :type Vector :default "0, 0, 0") (Hit :type Hit%20Result%20Structure%20%28by%20ref%29))
  ;[1 1 1] Cuando choco contra algo, si es un cuerpo físico, empujarlo... y si no, pues nada, ahí me quedo.
  (if (Physics|IsSimulatingPhysics OtherComp "None")
    (Utilities|IsValid OtherComp
      (:Is%20Valid
        (Physics|AddImpulseatLocation OtherComp (Transformation|GetVelocity) (Transformation|GetActorLocation) "None")))))

(fn ConstructionScript)